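; AI controller for RG units that turns player right-clicks into move targets.
; On BeginPlay it runs the BT_RGUnit behavior tree and binds to the player controller's right-mouse-button event.
; When a click misses the TraceTypeQuery3 cursor trace and the controlled unit is selected, it writes the Visibility-trace hit location to the TargetLocationToMove blackboard key.
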(event `self.ReceiveBeginPlay`
  (`self.RunBehaviorTree` "/Game/Entities/Units/AI/BT_RGUnit.BT_RGUnit")
  (bind _asbp_rgplayer_controller (cast `/Game/BP_RGPlayerController` (`GameplayStatics.GetPlayerController` 0)))
  (add `/Game/BP_RGPlayerController.RightMouseButtonPressed` _asbp_rgplayer_controller (delegate `RightMouseButtonPressedInteractableTrace`)))

(event `RightMouseButtonPressedInteractableTrace`
  (bind _returnvalue (`GameplayStatics.GetPlayerController` 0))
  (bind _returnvalue_2 (`self.K2_GetPawn` self))
  (if (not (`.ReturnValue` (`PlayerController.GetHitResultUnderCursorByChannel` _returnvalue "TraceTypeQuery3" true)))
    (bind _asrgunit_base (cast `RGUnitBase` _returnvalue_2))
    (if (`RGUnitBase.IsSelected` _asrgunit_base)
      (`BlackboardComponent.SetValueAsVector` (`AIBlueprintHelperLibrary.GetBlackboard` _returnvalue_2) "TargetLocationToMove" (`.Location` (`GameplayStatics.BreakHitResult` (`PlayerController.GetHitResultUnderCursorByChannel` _returnvalue "TraceTypeQuery1" true)))))))

(fn `UserConstructionScript`)